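; Farm plot that plants wheat, corn or pumpkin from the player's selected seed, grows it and yields a harvest actor.
; Planting uses up a seed, then swaps through three stage meshes, with a per-second Text3D countdown between stages.
; Each stage rolls for disease, which would halt growth with a diseased material, but its 1–100 roll below 1 never succeeds.
; Activar harvests grown crops, spawning the matching actor and freeing the plot.
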(event `Plantar Calabaza`
  (bind _relativetransformlocation (`self.RelativeTransformLocation`))
  (bind _returnvalue (`AddComponent|NODE_AddStaticMeshComponent-7` :`RelativeTransform` (`KismetMathLibrary.MakeTransform` _relativetransformlocation)))
  (`self.GrowTime` (`self.CalabazaCrecimiento`)
    (:`Salida`
      (`self.ChanceEnfermedad` _returnvalue
        (:`SinEnfermedad`
          (`ActorComponent.K2_DestroyComponent` _returnvalue)
          (bind _returnvalue_2 (`AddComponent|NODE_AddStaticMeshComponent-8` :`RelativeTransform` (`KismetMathLibrary.MakeTransform` _relativetransformlocation)))
          (`self.GrowTime` (`self.CalabazaCrecimiento`)
            (:`Salida`
              (`self.ChanceEnfermedad` _returnvalue_2
                (:`SinEnfermedad`
                  (`ActorComponent.K2_DestroyComponent` _returnvalue_2)
                  (bind _returnvalue_3 (`AddComponent|NODE_AddStaticMeshComponent-9` :`RelativeTransform` (`KismetMathLibrary.MakeTransform` _relativetransformlocation)))
                  (`self.ChanceEnfermedad` _returnvalue_3
                    (:`SinEnfermedad`
                      (set `self.YaCreció?` true)
                      (set `self.CurrentMesh` _returnvalue_3)
                      (set `self.QuePuedeCosecharse` "Calabaza"))))))))))))

(event `Plantar Elote`
  (bind _relativetransformlocation (`self.RelativeTransformLocation`))
  (bind _returnvalue (`AddComponent|NODE_AddStaticMeshComponent-4` :`RelativeTransform` (`KismetMathLibrary.MakeTransform` _relativetransformlocation)))
  (`self.GrowTime` (`self.EloteCrecimiento`)
    (:`Salida`
      (`self.ChanceEnfermedad` _returnvalue
        (:`SinEnfermedad`
          (`ActorComponent.K2_DestroyComponent` _returnvalue)
          (bind _returnvalue_2 (`AddComponent|NODE_AddStaticMeshComponent-5` :`RelativeTransform` (`KismetMathLibrary.MakeTransform` _relativetransformlocation)))
          (`self.GrowTime` (`self.EloteCrecimiento`)
            (:`Salida`
              (`self.ChanceEnfermedad` _returnvalue_2
                (:`SinEnfermedad`
                  (`ActorComponent.K2_DestroyComponent` _returnvalue_2)
                  (bind _returnvalue_3 (`AddComponent|NODE_AddStaticMeshComponent-6` :`RelativeTransform` (`KismetMathLibrary.MakeTransform` _relativetransformlocation)))
                  (`self.ChanceEnfermedad` _returnvalue_3
                    (:`SinEnfermedad`
                      (set `self.YaCreció?` true)
                      (set `self.CurrentMesh` _returnvalue_3)
                      (set `self.QuePuedeCosecharse` "Elote"))))))))))))

(event `Plantar Trigo`
  (bind _relativetransformlocation (`self.RelativeTransformLocation`))
  (bind _returnvalue (`AddComponent|NODE_AddStaticMeshComponent-0` :`RelativeTransform` (`KismetMathLibrary.MakeTransform` _relativetransformlocation)))
  (`self.GrowTime` (`self.TrigoCrecimiento`)
    (:`Salida`
      (`self.ChanceEnfermedad` _returnvalue
        (:`SinEnfermedad`
          (`ActorComponent.K2_DestroyComponent` _returnvalue)
          (bind _returnvalue_2 (`AddComponent|NODE_AddStaticMeshComponent-1` :`RelativeTransform` (`KismetMathLibrary.MakeTransform` _relativetransformlocation)))
          (`self.GrowTime` (`self.TrigoCrecimiento`)
            (:`Salida`
              (`self.ChanceEnfermedad` _returnvalue_2
                (:`SinEnfermedad`
                  (`ActorComponent.K2_DestroyComponent` _returnvalue_2)
                  (bind _returnvalue_3 (`AddComponent|NODE_AddStaticMeshComponent-2` :`RelativeTransform` (`KismetMathLibrary.MakeTransform` _relativetransformlocation)))
                  (`self.ChanceEnfermedad` _returnvalue_3
                    (:`SinEnfermedad`
                      (set `self.YaCreció?` true)
                      (set `self.CurrentMesh` _returnvalue_3)
                      (set `self.QuePuedeCosecharse` "Trigo"))))))))))))

(event `/Game/Blueprints/BP_Plantar.Plantar`
  (if (not (`self.HayAlgo?`))
    (bind _asthird_person_character (cast `/Game/ThirdPersonBP/Blueprints/ThirdPersonCharacter` (`GameplayStatics.GetPlayerCharacter` 0)))
    (switch `int` (`/Game/ThirdPersonBP/Blueprints/ThirdPersonCharacter.Semilla` _asthird_person_character)
      (:`0`
        (`self.TenemosSemillaTrigo`
          (:`Salida`
            (`self.Plantar Trigo`))))
      (:`1`
        (`self.TenemosSemillaElote`
          (:`Salida`
            (`self.Plantar Elote`))))
      (:`2`
        (`self.TenemosSemillaCalabaza`
          (:`Salida`
            (`self.Plantar Calabaza`)))))
    (set `self.HayAlgo?` true)))

(event `self.ReceiveBeginPlay`
  (`Text3DComponent.SetText` (`self.Text3D`) (`self.Value`)))

(event `/Game/Blueprints/BP_Activar. Activar`
  (`self.Cosechar`))

(fn `Cosechar`
  (bind _returnvalue (`KismetMathLibrary.Conv_VectorToTransform` (`SceneComponent.K2_GetComponentLocation` (`self.Text3D`))))
  (if (`self.YaCreció?`)
    (`ActorComponent.K2_DestroyComponent` (`self.CurrentMesh`))
    (switch `string` (`self.QuePuedeCosecharse`)
      (:`Default`
        _)
      (:`Trigo`
        (`|SpawnActorFromClass` "/Game/Blueprints/BP_TrigoCosecha.BP_TrigoCosecha_C" _returnvalue "Undefined" "OverrideRootScale" null null))
      (:`Elote`
        (`|SpawnActorFromClass` "/Game/Blueprints/BP_EloteCosecha.BP_EloteCosecha_C" _returnvalue "Undefined" "OverrideRootScale" null null))
      (:`Calabaza`
        (`|SpawnActorFromClass` "/Game/Blueprints/BP_CalabazaCosecha.BP_CalabazaCosecha_C" _returnvalue "Undefined" "OverrideRootScale" null null)))
    (set `self.YaCreció?` false)
    (set `self.CurrentMesh` null)
    (set `self.HayAlgo?` false)
    (set `self.QuePuedeCosecharse` "")))

(fn `UserConstructionScript`)